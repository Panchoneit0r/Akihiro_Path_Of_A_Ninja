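; BP_Door is a level gate that opens as samurai guards are defeated and triggers the victory screen.
; AddSamuraisDeafts counts defeats, hiding the door and disabling its collision at three, then showing WidgetBP_Victory with a mouse cursor after a delay from the fourth.
; When the third-person character hits the door, a delayed debug message says to defeat all guards.
; The character entering the Box trigger makes the Portal component blocking.
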(event `self.ReceiveActorBeginOverlap`
  (params (OtherActor :type "Actor Object Reference")))

(event `self.Door.OnComponentHit`
  (params (HitComponent :type "PrimitiveComponent Object Reference") (OtherActor :type "Actor Object Reference") (OtherComp :type "PrimitiveComponent Object Reference") (NormalImpulse :type "Vector Structure") (Hit :type "HitResult Structure (by ref)"))
  (cast `/Game/Characters/Ninja/BluePrints/BP_ThirdPersonCharacter` OtherActor)
  (`KismetSystemLibrary.Delay` 0.5)
  (`KismetSystemLibrary.PrintString` "Deaft all samurais guards"))

(event `AddSamuraisDeafts`
  (bind _door (`self.Door`))
  (bind _output_get (set `self.samuraisDeafts` (+ (`self.SamuraisDeafts`) 1)))
  (if (>= _output_get 3)
    (`SceneComponent.SetHiddenInGame` _door true false)
    (`PrimitiveComponent.SetCollisionProfileName` _door "NoCollision" true)
    (if (>= (`self.SamuraisDeafts`) 4)
      (`KismetSystemLibrary.Delay` 2.0)
      (bind _returnvalue (`|CreateWidget` "/Game/Widgets/Menu/WidgetBP_Victory.WidgetBP_Victory_C"))
      (`UserWidget.AddToViewport` _returnvalue 0)
      (`WidgetBlueprintLibrary.SetInputMode_GameAndUIEx` null null)
      (set `PlayerController.bShowMouseCursor` true (`GameplayStatics.GetPlayerController` 0)))))

(event `self.Box.OnComponentBeginOverlap`
  (params (OverlappedComponent :type "PrimitiveComponent Object Reference") (OtherActor :type "Actor Object Reference") (OtherComp :type "PrimitiveComponent Object Reference") (OtherBodyIndex :type Integer) (bFromSweep :type Boolean) (SweepResult :type "HitResult Structure (by ref)"))
  (cast `/Game/Characters/Ninja/BluePrints/BP_ThirdPersonCharacter` OtherActor)
  (`PrimitiveComponent.SetCollisionProfileName` (`self.Portal`) "BlockAllDynamic" true))

(fn `UserConstructionScript`)