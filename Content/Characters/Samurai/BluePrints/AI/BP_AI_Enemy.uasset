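; AI controller for enemies that runs their behavior tree and reacts to perceiving the player.
; On possess it caches the BP_EnemyDummy pawn and starts BT_Enemies.
; Perception updates for the third-person character set the IsPlayerSeeing blackboard key and drive a delayed loop that repeatedly calls AttackPlayer while the stimulus reads sensed.
; A FindPlayer move-to event exists, but its looping timer is disconnected.
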(event `self.ReceiveBeginPlay`)

(event `FindPlayer`
  (`|AIMoveTo` (`self.K2_GetPawn`) (0.0 0.0 0.0) (`GameplayStatics.GetPlayerController` 0)))

(event `self.ReceivePossess`
  (params (PossessedPawn :type "Pawn Object Reference"))
  (bind _asbp_enemy_dummy (cast `/Game/Characters/Samurai/BluePrints/BP_EnemyDummy` PossessedPawn))
  (`self.RunBehaviorTree` "/Game/Characters/Samurai/BluePrints/AI/BT_Enemies.BT_Enemies"))

(event `self.AIPerception.OnTargetPerceptionUpdated`
  (params (Actor :type "Actor Object Reference") (Stimulus :type "AIStimulus Structure"))
  (bind (_age _expirationage _strength _stimuluslocation _receiverlocation _tag _bsuccessfullysensed) (break `AIStimulus` Stimulus))
  (cast `/Game/Characters/Ninja/BluePrints/BP_ThirdPersonCharacter` Actor)
  (`BlackboardComponent.SetValueAsBool` (`self.Blackboard`) "IsPlayerSeeing" _bsuccessfullysensed)
  (if _bsuccessfullysensed :!label _label
    (`/Game/Characters/Samurai/BluePrints/BP_EnemyDummy.AttackPlayer` (stale `self.ReceivePossess` _asbp_enemy_dummy))
    (`KismetSystemLibrary.Delay` 0.5)
    (goto _label)))

(fn `UserConstructionScript`)