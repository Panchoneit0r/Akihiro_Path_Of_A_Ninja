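; BP_EnemyDummy is a samurai enemy that takes player damage, ragdolls on death and reports the kill to DoorLevel.
; Health lives in the overhead health bar widget, which yaws toward the player each tick.
; AttackPlayer plays a DoOnce-gated montage, and KattanaActivate toggles the katana box's overlap events to damage the player on contact.
; The pawn sensing handler is empty, and nothing live here calls AttackPlayer.
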(event `self.ReceiveBeginPlay`
  (bind _aswidget_bp_health_bar (cast `/Game/Widgets/Enemy/WidgetBP_HealthBar` (`WidgetComponent.GetUserWidgetObject` (`self.Widget`))))
  (bind _output_get (set `/Game/Widgets/Enemy/WidgetBP_HealthBar.MaxHealth` (`self.MaxHealth`) _aswidget_bp_health_bar))
  (set `/Game/Widgets/Enemy/WidgetBP_HealthBar.healt` _output_get _aswidget_bp_health_bar))

(event `TakeDamage`
  (params (PlayerDamage :type "Float (double-precision)"))
  (if (not (`self.death ?`))
    (bind _aswidget_bp_health_bar (cast `/Game/Widgets/Enemy/WidgetBP_HealthBar` (`WidgetComponent.GetUserWidgetObject` (`self.Widget`))))
    (set `/Game/Widgets/Enemy/WidgetBP_HealthBar.healt` (- (`/Game/Widgets/Enemy/WidgetBP_HealthBar.healt` _aswidget_bp_health_bar) PlayerDamage) _aswidget_bp_health_bar)
    (if (<= (`/Game/Widgets/Enemy/WidgetBP_HealthBar.healt` _aswidget_bp_health_bar) 0.0)
      (set `self.death ?` true)
      (`PrimitiveComponent.SetSimulatePhysics` (`self.Mesh`) true)
      (`SceneComponent.SetHiddenInGame` (`self.Widget`) true false)
      (`SceneComponent.SetHiddenInGame` (`self.Circle`) true false)
      (`/Game/Asian_Village/blueprints/BP_Door.AddSamuraisDeafts` (`self.DoorLevel`)))))

(event `self.ReceiveTick`
  (params (DeltaSeconds :type "Float (single-precision)"))
  (`SceneComponent.K2_SetWorldRotation` (`self.Widget`) (`KismetMathLibrary.MakeRotator` 0.0 0.0 (.yaw (`KismetMathLibrary.FindLookAtRotation` (`SceneComponent.K2_GetComponentLocation` (`self.Widget`)) (`self.K2_GetActorLocation` (`GameplayStatics.GetPlayerCharacter` 0))))) false false))

(event `AttackPlayer`
  (if (`self.PlayerLive ?`)
    (`/Engine/EditorBlueprintResources/StandardMacros.DoOnce` false :!label _label
      (:`Completed`
        (bind _returnvalue (`self.PlayAnimMontage` "/Game/Characters/Samurai/BluePrints/AnimBM_SamuraiWarriorAttack.AnimBM_SamuraiWarriorAttack" 1.5))
        (`KismetSystemLibrary.Delay` (/ _returnvalue 1.5))
        (goto _label :!via `Reset`)))))

(event `self.PawnSensing.OnSeePawn`
  (params (Pawn :type "Pawn Object Reference")))

(event `KattanaActivate`
  (bind _box (`self.Box`))
  ;[1 1 1] KatanaBoxFunctiopn
  (if (`PrimitiveComponent.bGenerateOverlapEvents` _box)
    (set `PrimitiveComponent.bGenerateOverlapEvents` false _box)
    (else
      (set `PrimitiveComponent.bGenerateOverlapEvents` true _box))))

(event `self.Box.OnComponentBeginOverlap`
  (params (OverlappedComponent :type "PrimitiveComponent Object Reference") (OtherActor :type "Actor Object Reference") (OtherComp :type "PrimitiveComponent Object Reference") (OtherBodyIndex :type Integer) (bFromSweep :type Boolean) (SweepResult :type "HitResult Structure (by ref)"))
  (bind _asbp_third_person_character (cast `/Game/Characters/Ninja/BluePrints/BP_ThirdPersonCharacter` OtherActor))
  (`/Game/Characters/Ninja/BluePrints/BP_ThirdPersonCharacter.DamagePlayer` _asbp_third_person_character 20.0)
  (set `self.PlayerLive ?` (>= (`/Game/Characters/Ninja/BluePrints/BP_ThirdPersonCharacter.Healt` _asbp_third_person_character) 0.0)))

(fn `UserConstructionScript`)